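; Lobby game mode that hosts a LAN dedicated-server session and moves players into the match map.
; BeginPlay creates the session through an Advanced Sessions node with a custom server-name setting and no presence, printing success or failure.
; PostLogin and HandleStartingNewPlayer call their parents and print each joining player.
; Once at least two players are present, the latter runs a servertravel console command to ThirdPersonExampleMap.
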(event `self.ReceiveBeginPlay`
  (`CreateSessionCallbackProxyAdvanced.CreateAdvancedSession` (`|MakeArray` (`AdvancedSessionsLibrary.MakeLiteralSessionPropertyString` "ServerName" "Namwook")) (`GameplayStatics.GetPlayerController` 0) 100 0 true true true false
    (:`OnSuccess`
      (`KismetSystemLibrary.PrintString` "세션생성성공"))
    (:`OnFailure`
      (`KismetSystemLibrary.PrintString` "세션생성실패"))))

(event `self.K2_PostLogin`
  (params (NewPlayer :type "PlayerController Object Reference"))
  (`parent.K2_PostLogin` null)
  (`KismetSystemLibrary.PrintString` (`KismetStringLibrary.Concat_StrStr` "On Post Login NewPlayer: " (`KismetSystemLibrary.GetDisplayName` NewPlayer)) true true (struct :`G` 0.66 :`B` 1.0 :`A` 1.0) 60.0))

(event `self.HandleStartingNewPlayer`
  (params (NewPlayer :type "PlayerController Object Reference"))
  (`parent.HandleStartingNewPlayer` NewPlayer)
  (`KismetSystemLibrary.PrintString` (`KismetStringLibrary.Concat_StrStr` "Handle Starting New Player: " (`KismetSystemLibrary.GetDisplayName` NewPlayer)) true true (struct :`G` 0.66 :`B` 1.0 :`A` 1.0) 60.0)
  (bind _returnvalue (`self.GetNumPlayers`))
  (if (>= _returnvalue 2)
    (`KismetSystemLibrary.ExecuteConsoleCommand` "servertravel ThirdPersonExampleMap" null)))

(fn `UserConstructionScript`)